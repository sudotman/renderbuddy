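; Actor Blueprint that recolors its static mesh using hex colors from a data table.
; At BeginPlay it creates a dynamic material instance on slot 0 and caches the table's "hex" column.
; UpdateColor recreates the material if invalid, then sets BaseColor from the cached hex entry at the DataAsset's Index, ignoring its own Index input.
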(event Custom|UpdateColor
  (params (index :type Integer))
  (Variables|Default|GetMaterialInstDynamic
    (:then
      _)
    (:else
      (CallFunction|CreateDynamicMaterial)))
  (bind _returnvalue (Class|MyBlueprintFunctionLibrary|HextoColor (Utilities|Array|Get(acopy) (Variables|Default|GetallColorsHex) (Variables|/Game/Blueprints/support/PrimaryIndexFetcher.PrimaryIndexFetcher_C|Getindex (Variables|Default|GetdataAsset)))))
  (Rendering|Material|SetVectorParameterValue (Variables|Default|GetMaterialInstDynamic) "BaseColor" (Math|Conversions|ToLinearColor(Color) _returnvalue) :!class /Script/Engine.MaterialInstanceDynamic))

(event Custom|CreateDynamicMaterial
  (bind _staticmeshcomponent (Variables|Debug|GetStaticMeshComponent))
  (bind _returnvalue (Rendering|Material|CreateDynamicMaterialInstance _staticmeshcomponent 0 (Rendering|Material|GetMaterial _staticmeshcomponent 0) "None" :!class /Script/Engine.PrimitiveComponent))
  (bind _output_get (Variables|Default|SetMaterialInstDynamic _returnvalue))
  (Rendering|Material|SetMaterial (Variables|Debug|GetStaticMeshComponent) 0 _output_get)
  (bind _returnvalue_2 (Class|DataTableFunctionLibrary|GetDataTableColumnasString "/Game/Blueprints/support/mainDataTable.mainDataTable" "hex"))
  (Variables|Default|SetallColorsHex _returnvalue_2))

(event EventBeginPlay
  (CallFunction|CreateDynamicMaterial))

(event Collision|EventActorBeginOverlap
  (params (OtherActor :type Actor%20Object%20Reference)))

(event EventTick
  (params (DeltaSeconds :type Float%20%28single-precision%29)))

(fn ConstructionScript)